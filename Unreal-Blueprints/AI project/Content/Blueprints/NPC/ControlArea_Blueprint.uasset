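; Control area actor that tracks which suspect Controlled_Object actors are inside it.
; Begin overlap casts to Controlled_Object, adds those flagged IsSuspect to SuspectsArray and sets AreSuspects.
; End overlap removes the leaving actor from the array.
; Tick polls the array and clears AreSuspects when it is empty.
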(event EventBeginPlay)

(event Collision|EventActorBeginOverlap
  (params (OtherActor :type Actor%20Object%20Reference))
  ;[1 1 1] Comprueba si hay sospechosos en el área, los añade al array de sospechosos y cambia la variable AreSuspects si no es true
  (bind _ascontrolled_object (Utilities|Casting|CastToControlled_Object OtherActor))
  (if (Variables|/Game/Blueprints/Controlled_Object.Controlled_Object_C|GetIsSuspect _ascontrolled_object)
    (Utilities|Array|Add (Variables|Default|GetSuspectsArray) OtherActor)
    (if (not (Variables|Default|GetAreSuspects))
      (Variables|Default|SetAreSuspects true))))

(event Collision|EventActorEndOverlap
  (params (OtherActor :type Actor%20Object%20Reference))
  ;[1 1 1] Cuando algún sospechoso sale del área se elimina
  (Utilities|Array|RemoveItem (Variables|Default|GetSuspectsArray) OtherActor))

(event EventTick
  (params (DeltaSeconds :type Float%20%28single-precision%29))
  ;[1 1 1] Si el array está vacío AreSuspects será false
  (if (== (Utilities|Array|Length (Variables|Default|GetSuspectsArray)) 0)
    (Variables|Default|SetAreSuspects false)))

(fn ConstructionScript)