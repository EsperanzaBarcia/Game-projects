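; Controlled_Object is a draggable cylinder actor randomly marked as suspect (red) or non-suspect (blue).
; The Construction Script rolls IsSuspect and applies the color through a dynamic material instance, so the roll repeats whenever construction reruns.
; Clicking the cylinder sets Clicked and opens a Gate on Tick, which moves the actor to the cursor's Camera-channel hit in X and Y, keeping Z.
; Releasing clears Clicked and closes the Gate.
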(event OnClicked(Cylinder)
  (params (TouchedComponent :type Primitive%20Component%20Object%20Reference) (ButtonPressed :type Key%20Structure :default "None"))
  (bind _returnvalue (Game|GetPlayerController 0))
  (bind _hitresult (Game|Player|GetHitResultUnderCursorbyChannel _returnvalue "TraceTypeQuery2" true))
  (bind _location (Collision|BreakHitResult _hitresult))
  (bind (_x _y) (Math|Vector|BreakVector _location))
  ;[1 1 1] Posicion del objeto
  (Variables|Default|SetClicked true)
  (Utilities|FlowControl|Gate true) ; enters at Open
)

(event OnReleased(Cylinder)
  (params (TouchedComponent :type Primitive%20Component%20Object%20Reference) (ButtonReleased :type Key%20Structure :default "None"))
  (bind _returnvalue (Game|GetPlayerController 0))
  (bind _hitresult (Game|Player|GetHitResultUnderCursorbyChannel _returnvalue "TraceTypeQuery2" true))
  (bind _location (Collision|BreakHitResult _hitresult))
  (bind (_x _y) (Math|Vector|BreakVector _location))
  ;[1 1 1] Posicion del objeto
  (Variables|Default|SetClicked false)
  (Utilities|FlowControl|Gate true) ; enters at Close
)

(event EventBeginPlay)

(event Collision|EventActorBeginOverlap
  (params (OtherActor :type Actor%20Object%20Reference)))

(event EventTick
  (params (DeltaSeconds :type Float%20%28single-precision%29))
  (bind _returnvalue (Game|GetPlayerController 0))
  (bind _hitresult (Game|Player|GetHitResultUnderCursorbyChannel _returnvalue "TraceTypeQuery2" true))
  (bind _location (Collision|BreakHitResult _hitresult))
  (bind (_x _y) (Math|Vector|BreakVector _location))
  ;[1 1 1] Posicion del objeto
  (Utilities|FlowControl|Gate true
    (:Exit
      (Transformation|SetActorLocation (Math|Vector|MakeVector _x _y (.Z (Math|Vector|BreakVector (Transformation|GetActorLocation)))) false false))))

(fn ConstructionScript
  ;[1 1 1] Selecciona el color del material según el valor (aleatorio) de la variable IsSuspect. Los sospechosos serán rojos y los no sospechosos azules
  (bind _output_get (Variables|Default|SetIsSuspect (Math|Random|RandomBool)))
  (if _output_get
    (Variables|Default|SetColor "(R=1.000000,G=0.000000,B=0.000000,A=1.000000)")
    (else
      (Variables|Default|SetColor "(R=0.000000,G=0.208099,B=0.658333,A=1.000000)")))
  ;[1 1 1] Cambio de material
  (bind _returnvalue (Rendering|Material|CreateDynamicMaterialInstance (Variables|Components|GetCylinder) 0 "/Game/Blueprints/ControlledObject_Material.ControlledObject_Material" "None" :!class /Script/Engine.PrimitiveComponent))
  (Variables|Default|SetMaterial _returnvalue)
  (Rendering|Material|SetVectorParameterValue _returnvalue "Color" (Variables|Default|GetColor) :!class /Script/Engine.MaterialInstanceDynamic))