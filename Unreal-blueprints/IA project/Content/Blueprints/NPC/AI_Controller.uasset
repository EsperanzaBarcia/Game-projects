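; AI controller for NPCs that patrol a control area and chase suspects found inside it.
; On BeginPlay it starts the behavior tree and blackboard, then cycles through the area's path points, writing each as TargetPos.
; A delayed event loop polls the ControlArea for suspects, setting the Suspect and Enemy keys to chase the first one, or clearing them to resume the route.
; Polling runs faster during a chase than on patrol.
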(event Custom|FollowEnemy
  (bind _bb (Variables|Default|GetBB))
  ;[1 1 1] Cambia los valores necesarios de la blackboard para que sea perseguido el sospechoso
  (AI|Components|Blackboard|SetValueasBool _bb (Variables|Default|GetSuspect) true)
  (AI|Components|Blackboard|SetValueasObject _bb (Variables|Default|GetEnemy) (stale Custom|Check%20area _suspect))
  (Utilities|FlowControl|Delay 0.2)
  (CallFunction|CheckArea))

(event Custom|Check%20area
  (bind _bb (Variables|Default|GetBB))
  ;[1 1 1] Comprueba si hay sospechosos, si es así se persigue al sospechoso. Si no, se sigue la ruta
  (bind (_suspects_boolean _suspect) (CallFunction|LookforSuspects))
  (if _suspects_boolean
    (CallFunction|FollowEnemy)
    (else
      (AI|Components|Blackboard|SetValueasBool _bb (Variables|Default|GetSuspect) false)
      (AI|Components|Blackboard|SetValueasObject _bb (Variables|Default|GetEnemy) 0)
      (CallFunction|FollowRoute))))

(event Custom|FollowRoute
  ;[1 1 1] Asigna las variables y cambia la target position de la blackboard para designar la siguiente posición
  ;;[1 1 1] Evento que permite avanzar en los path points
  (AI|Components|Blackboard|SetValueasVector (Variables|Default|GetBB) (Variables|Default|GetTargetPos) (+ (Transformation|GetActorLocation (Variables|/Game/Blueprints/NPC/AI_Character.AI_Character_C|GetControlArea (stale EventBeginPlay _asai_character))) (Utilities|Array|Get(acopy) (Variables|/Game/Blueprints/NPC/ControlArea_Blueprint.ControlArea_Blueprint_C|GetPathPoints (Variables|/Game/Blueprints/NPC/AI_Character.AI_Character_C|GetControlArea (stale EventBeginPlay _asai_character))) (Variables|Default|GetCurrentPathPointIndex))))
  (if (>= (Variables|Default|GetCurrentPathPointIndex) (Variables|Default|GetNumPathPoints))
    (Variables|Default|SetCurrentPathPointIndex 0)
    (else
      (Math|Integer|IncrementInt (Variables|Default|GetCurrentPathPointIndex)
        (:%20%20
          _))))
  (Utilities|FlowControl|Delay 2.0)
  (CallFunction|CheckArea))

(event EventBeginPlay
  ;[1 1 1] Asigna las variables y cambia la target position de la blackboard para designar la siguiente posición
  (bind _blackboardcomponent (Class|AIController|UseBlackboard "/Game/Blueprints/NPC/AI_BB.AI_BB"))
  (Variables|Default|SetBB _blackboardcomponent)
  (bind _asai_character (Utilities|Casting|CastToAI_Character (Pawn|GetControlledPawn self)))
  (Variables|Default|SetNumPathPoints (Utilities|Array|Length (Variables|/Game/Blueprints/NPC/ControlArea_Blueprint.ControlArea_Blueprint_C|GetPathPoints (Variables|/Game/Blueprints/NPC/AI_Character.AI_Character_C|GetControlArea _asai_character))))
  (AI|RunBehaviorTree "/Game/Blueprints/NPC/AI_BT.AI_BT")
  (AI|Components|Blackboard|SetValueasVector (Variables|Default|GetBB) (Variables|Default|GetTargetPos) (+ (Transformation|GetActorLocation (Variables|/Game/Blueprints/NPC/AI_Character.AI_Character_C|GetControlArea _asai_character)) (Utilities|Array|Get(acopy) (Variables|/Game/Blueprints/NPC/ControlArea_Blueprint.ControlArea_Blueprint_C|GetPathPoints (Variables|/Game/Blueprints/NPC/AI_Character.AI_Character_C|GetControlArea _asai_character)) (Variables|Default|GetCurrentPathPointIndex))))
  (if (>= (Variables|Default|GetCurrentPathPointIndex) (Variables|Default|GetNumPathPoints))
    (Variables|Default|SetCurrentPathPointIndex 0)
    (else
      (Math|Integer|IncrementInt (Variables|Default|GetCurrentPathPointIndex)
        (:%20%20
          _))))
  (Utilities|FlowControl|Delay 2.0)
  (CallFunction|CheckArea))

(fn ConstructionScript)

(fn LookforSuspects
  (bind _asai_character (Utilities|Casting|CastToAI_Character (Pawn|GetControlledPawn self)))
  (return (Variables|/Game/Blueprints/NPC/ControlArea_Blueprint.ControlArea_Blueprint_C|GetAreSuspects (Variables|/Game/Blueprints/NPC/AI_Character.AI_Character_C|GetControlArea _asai_character)) (Utilities|Array|Get(acopy) (Variables|/Game/Blueprints/NPC/ControlArea_Blueprint.ControlArea_Blueprint_C|GetSuspectsArray (Variables|/Game/Blueprints/NPC/AI_Character.AI_Character_C|GetControlArea _asai_character)))))